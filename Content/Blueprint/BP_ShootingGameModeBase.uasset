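; Game mode base for a shooting game that tracks the score and a persistent high score.
; On BeginPlay it shows the WBP_Score widget, hides the cursor, sets game-only input and loads the high score.
; AddScore accumulates points and, on a new record, saves it through a fresh BP_SaveGame object to a slot.
; Loading falls back to zero when the slot is missing or the cast fails.
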(event `self.ReceiveBeginPlay`
  (bind _returnvalue (`GameplayStatics.GetPlayerController` 0))
  ;[1 1 1] WBP_Score 화면에 출력
  ;;[1 1 1 1 12] Create Widget
  (bind _returnvalue_2 (`|CreateWidget` "/Game/Blueprint/WBP_Score.WBP_Score_C"))
  (`UserWidget.AddToViewport` _returnvalue_2 0)
  ;[1 1 1] 마우스 커서 숨김. 입력을 게임창에서 받음
  (set `PlayerController.bShowMouseCursor` false _returnvalue)
  (`WidgetBlueprintLibrary.SetInputMode_GameOnly` _returnvalue)
  (`self.LoadHighScore`))

(fn `AddScore`
  (params (Value :type Integer))
  ;[1 1 1] Score에 Value 누적, 만약 Score가 HighScore보다 크다면 HighScore에 Score값을 대입
  (bind _output_get (set `self.Score` (+ Value (`self.Score`))))
  (if (> _output_get (`self.HighScore`))
    (set `self.HighScore` _output_get)
    (`self.SaveHighScore`)))

(fn `LoadHighScore`
  ;[1 1 1] 저장 슬롯(파일)이 존재하는지 체크
  ; 슬롯을 읽어오면 SaveGame 객체를 반환
  ; BP_SaveGame으로 cast
  ; SaveHighScore를 HighScore에 대입
  (bind _returnvalue (`GameplayStatics.DoesSaveGameExist` (`self.SlotName`)))
  (if _returnvalue
    (bind _returnvalue_2 (`GameplayStatics.LoadGameFromSlot` (`self.SlotName`)))
    (bind _asbp_save_game (cast `/Game/Blueprint/BP_SaveGame` _returnvalue_2)
      (:`then`
        (set `self.HighScore` (`/Game/Blueprint/BP_SaveGame.SaveHighScore` _asbp_save_game)))
      (:`CastFailed`
        ;;[1 1 1] 없으면 0으로 세팅
        (set `self.HighScore` 0 :!label _label)))
    (else
      (goto _label))))

(fn `SaveHighScore`
  ;[1 1 1] SaveGame 객체를 만들고 그 객체의 속성에 저장할 값을 대입, 슬롯(파일)에 저장
  (`|ExecutionSequence`
    (:`then_0`
      (bind _returnvalue (`GameplayStatics.CreateSaveGameObject` "/Game/Blueprint/BP_SaveGame.BP_SaveGame_C"))
      (set `self.SaveGameInstance` _returnvalue))
    (:`then_1`
      (set `/Game/Blueprint/BP_SaveGame.SaveHighScore` (`self.HighScore`) (`self.SaveGameInstance`)))
    (:`then_2`
      (`GameplayStatics.SaveGameToSlot` (`self.SaveGameInstance`) (`self.SlotName`)))))

(fn `UserConstructionScript`)