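; BP_Enemy is an enemy actor that flies in a direction chosen at spawn and damages BP_Player on overlap.
; BeginPlay aims it at the player 30% of the time, otherwise along its forward vector; Tick moves and orients it along that direction through Translate.
; Overlap spawns explosion effects and calls the player's DoDamage.
; A true result destroys the player, pauses and shows WBP_GameOver; otherwise the enemy destroys itself.
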(event `self.ReceiveBeginPlay`
  ;[1 1 1] 태어날 때 방향 정하기. 30% 확률로 플레이어 향하는 방향 70% 아래 방향
  (if (< (`KismetMathLibrary.RandomIntegerInRange` 0 9) 3)
    ;;[1 1 1] 플레이어 찾아서 기억. 방향을 Direction변수에 대입
    (set `self.Direction` (`KismetMathLibrary.Normal` (- (`self.K2_GetActorLocation` (`GameplayStatics.GetPlayerPawn` 0)) (`self.K2_GetActorLocation`))))
    (else
      (set `self.Direction` (`self.GetActorForwardVector`)))))

(event `self.ReceiveActorBeginOverlap`
  (params (OtherActor :type "Actor Object Reference"))
  (bind _returnvalue (`GameplayStatics.GetPlayerController` 0))
  ;[1 1 1] 부딪힌 상대가 플레이어라면 부딪힌 위치에 복발 VFX를 표현하고 둘 다 죽음. Pause Game
  (bind _asbp_player (cast `/Game/Blueprint/BP_Player` OtherActor))
  (`GameplayStatics.SpawnEmitterAtLocation` "/Game/StarterContent/Particles/P_Explosion.P_Explosion" (`self.K2_GetActorLocation` _asbp_player))
  (`GameplayStatics.PlaySound2D` "/Game/Sound/Explosion.Explosion" 1.0 1.0 0.0 null null)
  (bind _isdie (`/Game/Blueprint/BP_Player.DoDamage` _asbp_player 10))
  (if _isdie
    (`self.K2_DestroyActor` _asbp_player)
    (`KismetSystemLibrary.Delay` 0.2)
    (`GameplayStatics.SetGamePaused` true)
    (bind _returnvalue_2 (`|CreateWidget` "/Game/Blueprint/WBP_GameOver.WBP_GameOver_C"))
    (`UserWidget.AddToViewport` _returnvalue_2 0)
    (set `PlayerController.bShowMouseCursor` true _returnvalue)
    (`WidgetBlueprintLibrary.SetInputMode_UIOnlyEx` _returnvalue null)
    (else
      (`self.K2_DestroyActor`))))

(event `self.ReceiveTick`
  (params (DeltaSeconds :type "Float (single-precision)"))
  ;[1 1 1] 살아가면서 정한 방향으로 이동
  (`self.Translate` (`self.Direction`) (`self.Speed`))
  (`self.K2_SetActorRotation` (`KismetMathLibrary.MakeRotFromXZ` (`self.Direction`) (`self.GetActorUpVector`))))

(fn `Translate`
  (params (Direction :type "Vector Structure") (Speed :type "Float (double-precision)") (IsSweep :type Boolean))
  (`self.K2_SetActorLocation` (+ (* (`KismetMathLibrary.Normal` Direction) Speed (`GameplayStatics.GetWorldDeltaSeconds`)) (`self.K2_GetActorLocation`)) IsSweep))

(fn `UserConstructionScript`)