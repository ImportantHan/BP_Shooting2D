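; BP_Player is the player-controlled shooter that moves along its right and up axes and fires BP_Bullet.
; Tick turns input axes into a normalized direction and moves the actor by speed and delta time, without sweep.
; Holding Fire runs a looping timer that spawns bullets at the Arrow with a sound, cleared on release.
; SetHP updates the WBP_PlayerHP widget; DoDamage subtracts health through it and reports death.
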(event `self.ReceiveBeginPlay`
  ;[1 1 1] 태어날 때 최대 체력 적용
  (`self.SetHP` (`self.MaxHP`)))

(event `self.ReceiveTick`
  (params (DeltaSeconds :type "Float (single-precision)"))
  (`|ExecutionSequence`
    (:`then_0`
      ;[1 1 1] 사용자의 입력에 따라 이동 p = p0 + vt
      (`self.Translate` (`self.GetDirection`) (`self.Speed`)))))

(event `InputAction|Fire`
  (params (Key :type "Key Structure"))
  ;[1 1 1] 마우스 왼쪽버튼 클릭 시 자동 발사
  (:`Pressed`
    (bind _returnvalue (`KismetSystemLibrary.K2_SetTimer` null "MakeBullet" (`self.FireInterval`) true))
    (set `self.MakeBulletTimerHandle` _returnvalue)
    (`self.MakeBullet`))
  (:`Released`
    (`KismetSystemLibrary.K2_ClearAndInvalidateTimerHandle` (`self.MakeBulletTimerHandle`))))

(fn `DoDamage`
  (params (Damage :type Integer))
  (returns (IsDie :type Boolean))
  ;[1 1 1] HP에서 Damage만큼 감소, 0이하일 경우 IsDie true
  (`self.SetHP` (- (`self.HP`) Damage))
  (if (<= (`self.HP`) 0)
    (return true)))

(fn `GetDirection`
  (returns (ReturnValue :type "Vector Structure"))
  (return (`KismetMathLibrary.Normal` (+ (* (`self.GetInputAxisValue`) (`self.GetActorRightVector`)) (* (`self.GetInputAxisValue`) (`self.GetActorUpVector`))))))

(fn `MakeBullet`
  (`|SpawnActorFromClass` "/Game/Blueprint/BP_Bullet.BP_Bullet_C" (`SceneComponent.K2_GetComponentToWorld` (`self.Arrow`)) "AlwaysSpawn" "MultiplyWithRoot" null null)
  (`GameplayStatics.PlaySound2D` "/Game/Sound/star-wars-blaster.star-wars-blaster" 1.0 1.0 0.0 null null))

(fn `SetHP`
  (params (Value :type Integer))
  (set `self.HP` Value)
  (bind _aswbp_player_hp (cast `/Game/Blueprint/WBP_PlayerHP` (`WidgetComponent.GetWidget` (`self.WidgetHP`))))
  (`/Game/Blueprint/WBP_PlayerHP.UpdateHP` _aswbp_player_hp (`KismetMathLibrary.Conv_IntToDouble` (`self.HP`)) (`KismetMathLibrary.Conv_IntToDouble` (`self.MaxHP`))))

(fn `Translate`
  (params (Direction :type "Vector Structure") (Speed :type "Float (double-precision)") (IsSweep :type Boolean))
  (`self.K2_SetActorLocation` (+ (* (`KismetMathLibrary.Normal` Direction) Speed (`GameplayStatics.GetWorldDeltaSeconds`)) (`self.K2_GetActorLocation`)) IsSweep))

(fn `UserConstructionScript`)