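; BP_Bullet is a projectile actor that destroys enemies it overlaps in a shooting game.
; Each tick, a Translate helper moves it along its forward vector by Speed times delta time, without sweep.
; Overlapping a BP_Enemy spawns an explosion at the enemy, destroys both actors, plays a sound, then adds a point through BP_ShootingGameModeBase.
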(event `self.ReceiveActorBeginOverlap`
  (params (OtherActor :type "Actor Object Reference"))
  ;[1 1 1] 총알 충돌 시 Enemy actor, Bullet actor destroy
  (bind _asbp_enemy (cast `/Game/Blueprint/BP_Enemy` OtherActor))
  (`GameplayStatics.SpawnEmitterAtLocation` "/Game/StarterContent/Particles/P_Explosion.P_Explosion" (`self.K2_GetActorLocation` _asbp_enemy))
  (`self.K2_DestroyActor` _asbp_enemy)
  (`self.K2_DestroyActor`)
  (`GameplayStatics.PlaySound2D` "/Game/Sound/Explosion.Explosion" 1.0 1.0 0.0 null null)
  (bind _asbp_shooting_game_mode_base (cast `/Game/Blueprint/BP_ShootingGameModeBase` (`GameplayStatics.GetGameMode`)))
  (`/Game/Blueprint/BP_ShootingGameModeBase.AddScore` _asbp_shooting_game_mode_base 1))

(event `self.ReceiveTick`
  (params (DeltaSeconds :type "Float (single-precision)"))
  ;[1 1 1] 나의 앞 방향으로 이동. p = p0 + vt
  (`self.Translate` (`self.GetActorForwardVector`) (`self.Speed`)))

(fn `Translate`
  (params (Direction :type "Vector Structure") (Speed :type "Float (double-precision)") (IsSweep :type Boolean))
  (`self.K2_SetActorLocation` (+ (* (`KismetMathLibrary.Normal` Direction) Speed (`GameplayStatics.GetWorldDeltaSeconds`)) (`self.K2_GetActorLocation`)) IsSweep))

(fn `UserConstructionScript`)