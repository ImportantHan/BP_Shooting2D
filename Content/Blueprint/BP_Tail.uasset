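; BP_Tail is an actor that follows a Target actor, defaulting to the player.
; On BeginPlay it keeps any preset Target, otherwise it stores the first BP_Player found in the level.
; Each Tick moves it along the normalized direction to the Target at Speed scaled by delta time, without sweep, stopping distance or a further validity check.
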(event `self.ReceiveBeginPlay`
  ;[1 1 1] 태어날 때 Target이 None일 경우 플레이어를 찾아서 목적지로 기억
  (`/Engine/EditorBlueprintResources/StandardMacros.IsValid` (`self.Target`)
    (:`Is Not Valid`
      (bind _returnvalue (`GameplayStatics.GetActorOfClass` "/Game/Blueprint/BP_Player.BP_Player_C"))
      (set `self.Target` _returnvalue))))

(event `self.ReceiveTick`
  (params (DeltaSeconds :type "Float (single-precision)"))
  ;[1 1 1] 목적지 향해 이동 (p += vt)
  ; Target - me : Target <- me
  ;;[1 1 1] vt
  (`self.K2_SetActorLocation` (+ (`self.K2_GetActorLocation`) (* (`self.Speed`) DeltaSeconds (`KismetMathLibrary.Normal` (- (`self.K2_GetActorLocation` (`self.Target`)) (`self.K2_GetActorLocation`)))))))

(fn `UserConstructionScript`)